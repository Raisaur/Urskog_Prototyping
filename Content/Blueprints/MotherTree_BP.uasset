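; MotherTree_BP is the Mother Tree actor, holding four sets of cameras, stairs and lights, apparently for staged reveals.
; BeginPlay groups these into arrays, hides the stairs, zeroes the lights and applies the first emissive level.
; Events drive stair opacity and tree glow through Material Parameter Collections, one per stair plus one for the tree.
; BlendCameratoPlayer ends a cinematic through the player character's cinematic widget, targeting the player.
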(event `self.ReceiveBeginPlay`
  (set `self.camera_actors_` (`|MakeArray` (`ChildActorComponent.ChildActor` (`self.FirstCameraActor`)) (`ChildActorComponent.ChildActor` (`self.SecondCameraActor`)) (`ChildActorComponent.ChildActor` (`self.ThirdCameraActor`)) (`ChildActorComponent.ChildActor` (`self.FourthCameraActor`))))
  (set `self.stairs_` (`|MakeArray` (`self.Stairs_First`) (`self.Stairs_Second`) (`self.Stairs_Third`) (`self.Stairs_Fourth`)))
  (bind _output_get (set `self.lights_` (`|MakeArray` (`self.Light_First`) (`self.Light_Second`) (`self.Light_Third`) (`self.Light_Fourth`))))
  (for (_array_element _array_index) _output_get
    (`self.SetStairOpacity` _array_index)
    (`LightComponent.SetIntensity` _array_element 0.0))
  (`KismetMaterialLibrary.SetScalarParameterValue` "/Game/Meshes/Mothertree/Textures/Mothertree_ParameterCollection.Mothertree_ParameterCollection" "emissive_" (`|GetArrayItem` (`self.mother_tree_emissive_`))))

(event `self.SetMotherTreeEmissive`
  (params (emisive :type "Float (single-precision)"))
  (`KismetMaterialLibrary.SetScalarParameterValue` "/Game/Meshes/Mothertree/Textures/Mothertree_ParameterCollection.Mothertree_ParameterCollection" "emissive_" emisive))

(event `self.SetStairOpacity`
  (params (index :type Integer) (opacity :type "Float (single-precision)"))
  (switch `int` index
    (:`Default`
      (`KismetSystemLibrary.PrintString` "No stairs, fall"))
    (:`0`
      (`KismetMaterialLibrary.SetScalarParameterValue` "/Game/Meshes/Mothertree/FirstStairParameterCollection.FirstStairParameterCollection" "opacity_" opacity))
    (:`1`
      (`KismetMaterialLibrary.SetScalarParameterValue` "/Game/Meshes/Mothertree/SecondStairParameterCollection.SecondStairParameterCollection" "opacity_" opacity))
    (:`2`
      (`KismetMaterialLibrary.SetScalarParameterValue` "/Game/Meshes/Mothertree/ThirdStairParameterCollectionCollection.ThirdStairParameterCollectionCollection" "opacity_" opacity))
    (:`3`
      (`KismetMaterialLibrary.SetScalarParameterValue` "/Game/Meshes/Mothertree/FourthStairParameterCollection.FourthStairParameterCollection" "opacity_" opacity))))

(event `self.BlendCameraToPlayer`
  (bind _cinematicwidget (`/Game/Blueprints/PlayerCharacter_BP.AddCinematicWidget` (cast `/Game/Blueprints/PlayerCharacter_BP` (`GameplayStatics.GetPlayerCharacter` 0) :!pure true)))
  (`/Game/HUD/CameraFade_BP.Init` _cinematicwidget true (`GameplayStatics.GetPlayerCharacter` 0) 2.0))

(fn `UserConstructionScript`)