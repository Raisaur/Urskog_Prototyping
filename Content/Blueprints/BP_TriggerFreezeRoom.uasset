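; BP_TriggerFreezeRoom is a trigger volume that shows the room-completed screen when the player enters it.
; A one-shot overlap on its collision component plays a 2D note sound, adds WBP_CompletedRoom to the viewport, and switches to UI-only input with a visible cursor.
; The DoOnce precedes the player cast, so the first overlap by any actor uses up the trigger.
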(event `self.CollisionComponent.OnComponentBeginOverlap`
  (params (OverlappedComponent :type "PrimitiveComponent Object Reference") (OtherActor :type "Actor Object Reference") (OtherComp :type "PrimitiveComponent Object Reference") (OtherBodyIndex :type Integer) (bFromSweep :type Boolean) (SweepResult :type "HitResult Structure (by ref)"))
  (bind _returnvalue (`GameplayStatics.GetPlayerController` 0))
  (`/Engine/EditorBlueprintResources/StandardMacros.DoOnce` false
    (:`Completed`
      (cast `/Game/Blueprints/PlayerCharacter_BP` OtherActor)
      (`GameplayStatics.PlaySound2D` "/Game/Audio/SC_Note_5.SC_Note_5" 1.0 1.0 0.0 null null)
      (bind _returnvalue_2 (`|CreateWidget` "/Game/UI/WBP_CompletedRoom.WBP_CompletedRoom_C" (`GameplayStatics.GetPlayerController` 0)))
      (set `self.WBP_CompletedRoom` _returnvalue_2)
      (`UserWidget.AddToViewport` (`self.WBP_CompletedRoom`) 0)
      (`WidgetBlueprintLibrary.SetInputMode_UIOnlyEx` _returnvalue (`self.WBP_CompletedRoom`))
      (set `PlayerController.bShowMouseCursor` true _returnvalue))))

(fn `UserConstructionScript`)