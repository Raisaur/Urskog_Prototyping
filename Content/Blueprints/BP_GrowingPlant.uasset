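; Plant actor that grows a flower once when Grow is called, with a particle effect shown during growth.
; Grow plays a non-looping skeletal animation, shows the particles and sets a flag that blocks repeat calls.
; Tick then runs a hardcoded five-second timer before DoneGrowing hides the particles and ticking is disabled.
; An animation-Blueprint completion check remains in the graph but is disconnected.
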(event `self.ReceiveBeginPlay`)

(event `self.ReceiveTick`
  (params (DeltaSeconds :type "Float (single-precision)"))
  (if (`self.growing`)
    (bind _output_get (set `self.Timer` (+ DeltaSeconds (`self.Timer`))))
    (if (>= _output_get 5.0)
      (`self.DoneGrowing`)
      (`self.SetActorTickEnabled` false))))

(fn `DoneGrowing`
  (`SceneComponent.SetVisibility` (`self.ParticleSystem`) false false))

(fn `Grow`
  (if (not (`self.growing`))
    (`SkeletalMeshComponent.PlayAnimation` (`self.SkeletalMesh`) "/Game/Meshes/GrowingFlower/SK_GrowingFLower_Anim.SK_GrowingFLower_Anim" false)
    (`SceneComponent.SetVisibility` (`self.ParticleSystem`) true false)
    (set `self.growing` true)))

(fn `UserConstructionScript`)