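; First-person-style player character with movement, run, jump, item pickup/placement and four selectable abilities: grow plants, freeze, light and wind.
; Camera line traces target plants, spawn or remove a capped list of ice blocks, and move items through an InventoryCam_BP actor.
; While lit, the spotlight tracks the aim point each tick, scales intensity by distance and charges light crystals.
; Wind flags BP_PushObjects via Windbeam overlaps; Gust's impulse logic is disconnected.
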(event `self.ReceiveBeginPlay`
  (bind _charactermovement (`self.CharacterMovement`))
  (set `CharacterMovementComponent.JumpZVelocity` 800.0 _charactermovement)
  (set `CharacterMovementComponent.GravityScale` 2.0 _charactermovement)
  (bind _returnvalue (`GameplayStatics.GetActorOfClass` "/Game/Blueprints/InventoryCam_BP.InventoryCam_BP_C"))
  (set `self.inventory_camera_` _returnvalue)
  (set `self.base_light_intensity_` (`LightComponentBase.Intensity` (`self.SpotLight`))))

(event `self.ReceiveTick`
  (params (DeltaSeconds :type "Float (single-precision)"))
  (`self.UpdateLight`)
  (`self.Gust`))

(event `InputAxis|MoveForward`
  (params (AxisValue :type "Float (single-precision)"))
  ;[1 1 1] Movement and Camera
  (`self.AddMovementInput` (`self.GetActorForwardVector`) AxisValue))

(event `InputAction|UseAbility`
  (params (Key :type "Key Structure"))
  ;[1 1 1] Actions
  (:`Pressed`
    (`self.Use Ability`))
  (:`Released`
    (`self.StopUsingAbility`)))

(event `InputAxis|MoveRight`
  (params (AxisValue :type "Float (single-precision)"))
  ;[1 1 1] Movement and Camera
  (`self.AddMovementInput` (`self.GetActorRightVector`) AxisValue))

(event `InputAction|PickUp/Place`
  (params (Key :type "Key Structure"))
  ;[1 1 1] Actions
  (:`Pressed`
    (`self.PickUp/Place`)))

(event `InputAxis|LookUp`
  (params (AxisValue :type "Float (single-precision)"))
  ;[1 1 1] Movement and Camera
  (`self.AddControllerPitchInput` AxisValue))

(event `InputAxis|Turn`
  (params (AxisValue :type "Float (single-precision)"))
  ;[1 1 1] Movement and Camera
  (`self.AddControllerYawInput` AxisValue))

(event `InputAction|Jump`
  (params (Key :type "Key Structure"))
  ;[1 1 1] Movement and Camera
  (:`Pressed`
    (`self.Jump`))
  (:`Released`
    (`self.StopJumping`)))

(event `InputAction|Run`
  (params (Key :type "Key Structure"))
  (bind _charactermovement (`self.CharacterMovement`))
  ;[1 1 1] Movement and Camera
  (:`Pressed`
    (set `CharacterMovementComponent.MaxWalkSpeed` (`self.run_speed_`) _charactermovement))
  (:`Released`
    (set `CharacterMovementComponent.MaxWalkSpeed` (`self.walk_speed_`) _charactermovement)))

(event `self.Windbeam.OnComponentBeginOverlap`
  (params (OverlappedComponent :type "PrimitiveComponent Object Reference") (OtherActor :type "Actor Object Reference") (OtherComp :type "PrimitiveComponent Object Reference") (OtherBodyIndex :type Integer) (bFromSweep :type Boolean) (SweepResult :type "HitResult Structure (by ref)"))
  (bind _asbp_push_object (cast `/Game/Blueprints/Interactables/Bp_PushObject` OtherActor))
  (set `/Game/Blueprints/Interactables/Bp_PushObject.being_pushed_` true _asbp_push_object))

(event `self.Windbeam.OnComponentEndOverlap`
  (params (OverlappedComponent :type "PrimitiveComponent Object Reference") (OtherActor :type "Actor Object Reference") (OtherComp :type "PrimitiveComponent Object Reference") (OtherBodyIndex :type Integer))
  (bind _asbp_push_object (cast `/Game/Blueprints/Interactables/Bp_PushObject` OtherActor))
  (set `/Game/Blueprints/Interactables/Bp_PushObject.being_pushed_` false _asbp_push_object))

(fn `EndWind`
  (set `self.wind_active_` false)
  (set `PrimitiveComponent.bGenerateOverlapEvents` false (`self.Windbeam`)))

(fn `Freeze`
  (bind _returnvalue (`SceneComponent.GetForwardVector` (`self.Camera`)))
  (bind (_hitresult _hit) (`self.SingleLineTrace` 200.0))
  (bind _asbp_ice_object (cast `/Game/Blueprints/Interactables/BP_IceObject` (`.HitActor` (`GameplayStatics.BreakHitResult` _hitresult)))
    (:`then`
      (`self.RemoveIce` _asbp_ice_object))
    (:`CastFailed`
      (bind _returnvalue_2 (`|SpawnActorFromClass` "/Game/Blueprints/Interactables/BP_IceObject.BP_IceObject_C" (`KismetMathLibrary.MakeTransform` (+ (`KismetMathLibrary.SelectVector` (* _returnvalue (`.Distance` (`GameplayStatics.BreakHitResult` _hitresult))) (* _returnvalue 400.0) _hit) (`self.K2_GetActorLocation`))) "Undefined" "OverrideRootScale" null null))
      (`KismetArrayLibrary.Array_AddUnique` (`self.ice_objects_`) _returnvalue_2)
      (bind (_returnvalue_x _returnvalue_y _returnvalue_z) (`KismetMathLibrary.BreakVector` (`SceneComponent.K2_GetComponentLocation` (`/Game/Blueprints/Interactables/BP_IceObject.StaticMesh` _returnvalue_2))))
      (`SceneComponent.K2_SetWorldLocation` (`/Game/Blueprints/Interactables/BP_IceObject.StaticMesh` _returnvalue_2) (`KismetMathLibrary.MakeVector` _returnvalue_x _returnvalue_y (+ _returnvalue_z (.z (`.BoxExtent` (`self.GetActorBounds` _returnvalue_2 false false))))) false false)
      (if (> (`KismetArrayLibrary.Array_Length` (`self.ice_objects_`)) (`self.max_ice_objects_`))
        (`self.RemoveIce` (`|GetArrayItem` (`self.ice_objects_`)))))))

(fn `Grow`
  (bind _hitresult (`self.SingleLineTrace` 1000.0))
  (bind _asbp_growing_plant (cast `/Game/Blueprints/BP_GrowingPlant` (`.HitActor` (`GameplayStatics.BreakHitResult` _hitresult))))
  (`/Game/Blueprints/BP_GrowingPlant.Grow` _asbp_growing_plant))

(fn `Gust`)

(fn `Light`
  (`SceneComponent.SetVisibility` (`self.SpotLight`) true false)
  (set `self.update_light_` true))

(fn `PickUp`
  (bind _hitresult (`self.SingleLineTrace` 1000.0))
  (bind _aspick_up_object_bp (cast `/Game/Blueprints/Interactables/PickUpObject_BP` (`.HitActor` (`GameplayStatics.BreakHitResult` _hitresult))))
  (`/Game/Blueprints/InventoryCam_BP.SetTargetObject` (`self.inventory_camera_`) _aspick_up_object_bp))

(fn `PickUp/Place`
  (if (`/Game/Blueprints/InventoryCam_BP.HasTarget` (`self.inventory_camera_`))
    (`self.Place`)
    (else
      (`self.PickUp`))))

(fn `Place`
  (bind _hitresult (`self.SingleLineTrace` (`self.place_distance_`)))
  (if (`GameplayStatics.BreakHitResult` _hitresult)
    (`/Game/Blueprints/InventoryCam_BP.PlaceTarget` (`self.inventory_camera_`) (`KismetMathLibrary.MakeTransform` (`.ImpactPoint` (`GameplayStatics.BreakHitResult` _hitresult))))))

(fn `RemoveIce`
  (params (Ice :type "/Game/Blueprints/Interactables/BP_IceObject Object Reference"))
  (`self.K2_DestroyActor` Ice)
  (`KismetArrayLibrary.Array_RemoveItem` (`self.ice_objects_`) Ice))

(fn `SetAbility`
  (params (AbilityNr :type Integer))
  (`self.StopUsingAbility`)
  (set `self.selected_ability_nr_` AbilityNr))

(fn `SingleLineTrace`
  (params (distance :type "Float (double-precision)" :default 1000.0))
  (returns (HitResult :type "HitResult Structure") (Hit :type Boolean))
  (bind _camera (`self.Camera`))
  (bind _returnvalue (`SceneComponent.K2_GetComponentLocation` _camera))
  (bind (_outhit _returnvalue_2) (`KismetSystemLibrary.LineTraceSingle` _returnvalue (+ _returnvalue (* (`SceneComponent.GetForwardVector` _camera) distance)) "TraceTypeQuery1"))
  (return _outhit _returnvalue_2))

(fn `StartWind`
  (set `self.wind_active_` true)
  (set `PrimitiveComponent.bGenerateOverlapEvents` true (`self.Windbeam`)))

(fn `StopLight`
  (`SceneComponent.SetVisibility` (`self.SpotLight`) false false)
  (set `self.update_light_` false))

(fn `StopUsingAbility`
  (switch `int` (`self.selected_ability_nr_`)
    (:`3`
      (`self.StopLight`))
    (:`4`
      (`self.EndWind`))))

(fn `UpdateLight`
  (bind _base_light_intensity_ (`self.base_light_intensity_`))
  (if (`self.update_light_`)
    (bind (_hitresult _hit) (`self.SingleLineTrace` 1000.0))
    (`SceneComponent.K2_SetWorldRotation` (`self.SpotLight`) (`KismetMathLibrary.FindLookAtRotation` (`SceneComponent.K2_GetComponentLocation` (`self.SpotLight`)) (`KismetMathLibrary.SelectVector` (`.Location` (`GameplayStatics.BreakHitResult` _hitresult)) (`.TraceEnd` (`GameplayStatics.BreakHitResult` _hitresult)) _hit)) false false)
    (if _hit
      (`LightComponent.SetIntensity` (`self.SpotLight`) (`KismetMathLibrary.FClamp` (* (/ (`.Distance` (`GameplayStatics.BreakHitResult` _hitresult)) 1000.0) _base_light_intensity_) (* _base_light_intensity_ 0.1) _base_light_intensity_))
      (bind _asbp_light_crystal (cast `/Game/Blueprints/Interactables/BP_LightCrystal` (`.HitActor` (`GameplayStatics.BreakHitResult` _hitresult))))
      (`/Game/Blueprints/Interactables/BP_LightCrystal.IncreaseLight` _asbp_light_crystal)
      (else
        (`LightComponent.SetIntensity` (`self.SpotLight`) (`self.base_light_intensity_`))))))

(fn `Use Ability`
  ;[1 1 1] ability 0 is no ability
  (switch `int` (`self.selected_ability_nr_`)
    (:`1`
      (`self.Grow`))
    (:`2`
      (`self.Freeze`))
    (:`3`
      (`self.Light`))
    (:`4`
      (`self.StartWind`))))

(fn `UserConstructionScript`)