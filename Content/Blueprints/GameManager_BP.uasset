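; GameManager_BP is a game manager that updates the easter egg counter UI and runs the end credits sequence.
; The easter egg event plays the gameplay widget's animation with the activated count, lazily fetching and caching that widget from the player character when it is invalid.
; Starting credits clears all widgets, spawns a wisp, blends the view to the credits camera, then shows the credits widget after a delay matching the blend.
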(event `self.SetEasterEggCountUI`
  (`/Engine/EditorBlueprintResources/StandardMacros.IsValid` (`self.gameplay_widget`)
    (:`Is Valid`
      _)
    (:`Is Not Valid`
      (bind _asplayer_character_bp (cast `/Game/Blueprints/PlayerCharacter_BP` (`GameplayStatics.GetPlayerCharacter` 0)))
      (set `self.gameplay_widget` (`/Game/Blueprints/PlayerCharacter_BP.gameplay_widget` _asplayer_character_bp))))
  (`/Game/HUD/Gameplay_BP.PlayEasterEggAnimation` (`self.gameplay_widget`) (`self.activated_easter_egg_count_`)))

(event `self.StartCredits`
  (`WidgetLayoutLibrary.RemoveAllWidgets`)
  (`self.SpawnWisp`)
  (`PlayerController.SetViewTargetWithBlend` (`GameplayStatics.GetPlayerController` 0) (`self.credits_camera_`) 2.0 "VTBlend_Linear" 0.0 false)
  (`KismetSystemLibrary.Delay` 2.0)
  (bind _returnvalue (`|CreateWidget` "/Game/HUD/CreditWidget_BP.CreditWidget_BP_C"))
  (`UserWidget.AddToViewport` _returnvalue 0))

(fn `UserConstructionScript`)