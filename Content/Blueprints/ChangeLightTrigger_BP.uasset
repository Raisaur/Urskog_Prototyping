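; Light-change trigger Blueprint that blends the level's BP_Sky_Sphere toward target sky settings over a lerp time.
; One event snapshots the current zenith and horizon colors, star and sun brightness, and cloud opacity.
; Another interpolates each toward its target by Timer / LerpTime and refreshes the sky material; neither timer updates nor trigger detection appear here.
; GetSkySphere lazily finds and caches the sky actor.
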(event `self.LerpSkySphereValues`
  (bind _returnvalue (/ (`self.timer_`) (`self.lerp_time_`)))
  (`|ExecutionSequence`
    (:`then_0`
      (bind _newparam (`self.GetSkySphere`))
      (set `/Engine/EngineSky/BP_Sky_Sphere.Zenith Color` (`KismetMathLibrary.LinearColorLerp` (`self.initial_zenith_color_`) (`self.zenith_color_`) _returnvalue) _newparam))
    (:`then_1`
      (bind _newparam_2 (`self.GetSkySphere`))
      (set `/Engine/EngineSky/BP_Sky_Sphere.Horizon color` (`KismetMathLibrary.LinearColorLerp` (`self.initial_horizon_color_`) (`self.horizon_color_`) _returnvalue) _newparam_2))
    (:`then_2`
      (bind _newparam_3 (`self.GetSkySphere`))
      (set `/Engine/EngineSky/BP_Sky_Sphere.Stars brightness` (`KismetMathLibrary.Lerp` (`self.initial_star_brightness_`) (`self.star_brightness_`) _returnvalue) _newparam_3))
    (:`then_3`
      (bind _newparam_4 (`self.GetSkySphere`))
      (set `/Engine/EngineSky/BP_Sky_Sphere.Sun brightness` (`KismetMathLibrary.Lerp` (`self.initial_sun_brightness`) (`self.sun_brightness_`) _returnvalue) _newparam_4))
    (:`then_4`
      (bind _newparam_5 (`self.GetSkySphere`))
      (set `/Engine/EngineSky/BP_Sky_Sphere.Cloud opacity` (`KismetMathLibrary.Lerp` (`self.initial_cloud_opacity_`) (`self.cloud_opacity_`) _returnvalue) _newparam_5))
    (:`then_5`
      (bind _newparam_6 (`self.GetSkySphere`))
      (`/Engine/EngineSky/BP_Sky_Sphere.RefreshMaterial` _newparam_6))))

(event `self.SetSkySphereInitialValues`
  (bind _newparam (`self.GetSkySphere`))
  (set `self.initial_zenith_color_` (`/Engine/EngineSky/BP_Sky_Sphere.Zenith Color` _newparam))
  (set `self.initial_horizon_color_` (`/Engine/EngineSky/BP_Sky_Sphere.Horizon color` _newparam))
  (set `self.initial_star_brightness_` (`/Engine/EngineSky/BP_Sky_Sphere.Stars brightness` _newparam))
  (set `self.initial_sun_brightness` (`/Engine/EngineSky/BP_Sky_Sphere.Sun brightness` _newparam))
  (set `self.initial_cloud_opacity_` (`/Engine/EngineSky/BP_Sky_Sphere.Cloud opacity` _newparam)))

(fn `GetSkySphere`
  (returns (NewParam :type "/Engine/EngineSky/BP_Sky_Sphere Object Reference"))
  (bind _sky_sphere (`self.sky_sphere`))
  (`/Engine/EditorBlueprintResources/StandardMacros.IsValid` _sky_sphere
    (:`Is Valid`
      (return _sky_sphere))
    (:`Is Not Valid`
      (bind _returnvalue (`GameplayStatics.GetActorOfClass` "/Engine/EngineSky/BP_Sky_Sphere.BP_Sky_Sphere_C"))
      (bind _output_get (set `self.sky_sphere` _returnvalue))
      (return _output_get))))

(fn `UserConstructionScript`)