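; Grid Blueprint that classifies a tile by what overlaps its box, through the CheckTileOverlap event.
; Nested box overlap queries on two custom object channels give the tile one type for either channel alone and another for both, via SetTileType.
; A WorldStatic overlap then overrides that type with a fourth one.
; Tiles touching neither custom channel skip the WorldStatic test and keep their current type.
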(event `self.CheckTileOverlap`
  (params (tile_to_check_ :type "Tile Structure"))
  (bind (_index_ _position_ _tile_type_ _extent_) (break `Tile` tile_to_check_))
  (bind _array (`|MakeArray` "ObjectTypeQuery10" :!type "EObjectTypeQuery Enum"))
  (bind (_outactors _returnvalue) (`KismetSystemLibrary.BoxOverlapActors` _position_ _extent_ (`|MakeArray` "ObjectTypeQuery9" :!type "EObjectTypeQuery Enum")))
  (if _returnvalue
    (bind (_outactors_2 _returnvalue_2) (`KismetSystemLibrary.BoxOverlapActors` _position_ _extent_ _array))
    (if _returnvalue_2
      (`self.SetTileType` _index_ 2)
      (else
        (`self.SetTileType` _index_)))
    (bind (_outactors_3 _returnvalue_3) (`KismetSystemLibrary.BoxOverlapActors` _position_ _extent_ (`|MakeArray` "ObjectTypeQuery1" :!type "EObjectTypeQuery Enum") :!label _label))
    (if _returnvalue_3
      (`self.SetTileType` _index_ 3))
    (else
      (bind (_outactors_4 _returnvalue_4) (`KismetSystemLibrary.BoxOverlapActors` _position_ _extent_ _array))
      (if _returnvalue_4
        (`self.SetTileType` _index_ 1)
        (goto _label)))))

(fn `UserConstructionScript`)