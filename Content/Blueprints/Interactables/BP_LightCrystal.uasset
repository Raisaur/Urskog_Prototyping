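; BP_LightCrystal is a crystal actor that brightens when IncreaseLight is called and dims again after a delay.
; BeginPlay applies a dynamic M_Crystal material instance to the mesh, whose emissive parameter drives the glow.
; IncreaseLight steps emissive up to a cap and resets the timer only when that step succeeds.
; Once the timer exceeds TimeToUnlit, Tick calls DecreaseLight every frame, stepping emissive down toward a floor.
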(event `self.ReceiveBeginPlay`
  (bind _returnvalue (`KismetMaterialLibrary.CreateDynamicMaterialInstance` "/Game/Meshes/PrototypeRoom/Crystal/M_Crystal.M_Crystal"))
  (bind _output_get (set `self.material_` _returnvalue))
  (`PrimitiveComponent.SetMaterial` (`self.StaticMesh`) 0 _output_get))

(event `self.ReceiveTick`
  (params (DeltaSeconds :type "Float (single-precision)"))
  (bind _output_get (set `self.timer` (+ DeltaSeconds (`self.timer`))))
  (if (not (not (> _output_get (`self.time_to_unlit_`))))
    (`self.DecreaseLight`)))

(fn `DecreaseLight`
  (bind _returnvalue (- (`self.emissive_value_`) (`self.emissive_decrement_`)))
  (if (not (< _returnvalue 1.0))
    (bind _output_get (set `self.emissive_value_` _returnvalue))
    (`MaterialInstanceDynamic.SetScalarParameterValue` (`self.material_`) "Emissive_" _output_get)))

(fn `IncreaseLight`
  (bind _returnvalue (+ (`self.emissive_value_`) (`self.emissive_increment_`)))
  (if (not (> _returnvalue 10.0))
    (bind _output_get (set `self.emissive_value_` _returnvalue))
    (`MaterialInstanceDynamic.SetScalarParameterValue` (`self.material_`) "Emissive_" _output_get)
    (set `self.timer` 0.0)))

(fn `UserConstructionScript`)