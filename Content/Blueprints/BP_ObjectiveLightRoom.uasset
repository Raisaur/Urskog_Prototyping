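; BP_ObjectiveLightRoom is a collectible key part for a light room objective, with a completion check.
; Overlapping KeyPartMesh adds to the player's light-part total, plays a sound and destroys the actor.
; The first Sphere overlap, gated by DoOnce before the player cast, compares that total to the required amount.
; When met, it shows WBP_CompletedRoom with a sound, UI-only input and mouse cursor.
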(event `self.KeyPartMesh.OnComponentBeginOverlap`
  (params (OverlappedComponent :type "PrimitiveComponent Object Reference") (OtherActor :type "Actor Object Reference") (OtherComp :type "PrimitiveComponent Object Reference") (OtherBodyIndex :type Integer) (bFromSweep :type Boolean) (SweepResult :type "HitResult Structure (by ref)"))
  ;[1 1 1] Gathering the objective
  (bind _asplayer_character_bp (cast `/Game/Blueprints/PlayerCharacter_BP` OtherActor))
  (bind _output_get (set `/Game/Blueprints/PlayerCharacter_BP.KeyPart_TotalAmountLight` (+ (`/Game/Blueprints/PlayerCharacter_BP.KeyPart_TotalAmountLight` _asplayer_character_bp) (`self.KeyPart_SingleLight`)) _asplayer_character_bp))
  (`KismetSystemLibrary.PrintString` (`KismetStringLibrary.Conv_IntToString` _output_get))
  (`GameplayStatics.PlaySound2D` "/Game/Audio/SC_Note_5.SC_Note_5" 1.0 1.0 0.0 null null)
  (`self.K2_DestroyActor`))

(event `self.Sphere.OnComponentBeginOverlap`
  (params (OverlappedComponent :type "PrimitiveComponent Object Reference") (OtherActor :type "Actor Object Reference") (OtherComp :type "PrimitiveComponent Object Reference") (OtherBodyIndex :type Integer) (bFromSweep :type Boolean) (SweepResult :type "HitResult Structure (by ref)"))
  (bind _returnvalue (`GameplayStatics.GetPlayerController` 0))
  ;[1 1 1] Completing to gather all the objectives, making a widget popping up.
  (`/Engine/EditorBlueprintResources/StandardMacros.DoOnce` false
    (:`Completed`
      (bind _asplayer_character_bp (cast `/Game/Blueprints/PlayerCharacter_BP` OtherActor))
      (if (>= (`/Game/Blueprints/PlayerCharacter_BP.KeyPart_TotalAmountLight` _asplayer_character_bp) (`self.KeyParts_RequiredAmountLight`))
        (`GameplayStatics.PlaySound2D` "/Game/Audio/SC_Note_5.SC_Note_5" 1.0 1.0 0.0 null null)
        (bind _returnvalue_2 (`|CreateWidget` "/Game/UI/WBP_CompletedRoom.WBP_CompletedRoom_C" (`GameplayStatics.GetPlayerController` 0)))
        (set `self.WBP_CompletedRoom` _returnvalue_2)
        (`UserWidget.AddToViewport` (`self.WBP_CompletedRoom`) 0)
        (`WidgetBlueprintLibrary.SetInputMode_UIOnlyEx` _returnvalue (`self.WBP_CompletedRoom`))
        (set `PlayerController.bShowMouseCursor` true _returnvalue)))))

(fn `UserConstructionScript`)