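; Trigger actor that shows a controls popup the first time a qualifying actor overlaps it.
; On overlap, a cast filters the other actor, then the popup widget is initialized with keyboard-mouse and gamepad images, an action name, and primary and secondary keys.
; The widget is added to the viewport if not already shown, and a once flag blocks repeats after a valid popup is handled.
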(event `self.ReceiveActorBeginOverlap`
  (params (OtherActor :type "Actor Object Reference"))
  (bind _controls_popup_ (`self.controls_popup_`))
  (if (`self.b_once`)
    _
    (elif (cast `` OtherActor :!pure true)
      (`/Engine/EditorBlueprintResources/StandardMacros.IsValid` (`self.controls_popup_`)
        (:`Is Valid`
          (`/Game/HUD/ControlsPopUp_BP.Init` (`self.controls_popup_`) (`self.kbm_image`) (`self.gp_image`) (`self.action_name_`) (`self.primary_key_`) (`self.secondary_key_`))
          (if (not (`Widget.IsInViewport` _controls_popup_))
            (`UserWidget.AddToViewport` _controls_popup_ 0))
          (set `self.b_once` true))))))

(fn `UserConstructionScript`)