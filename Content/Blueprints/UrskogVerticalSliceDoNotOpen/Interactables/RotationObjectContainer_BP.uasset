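; RotationObjectContainer_BP is an interactable container that groups three rotation objects placed as child actor components.
; Its construction script casts the three child actors, stopping if any cast fails, then adds all three to the RotationObjects array and clamps NumberOfRotationObjects to that count.
; It then calls SetInitialRotations and SetRotationPerInteraction, whose logic is not included here, to configure the objects' rotations.
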(fn `UserConstructionScript`
  (bind _asrotate_object (cast `` (`ChildActorComponent.ChildActor` (`self.RotationObject_1`))))
  (bind _asrotate_object_2 (cast `` (`ChildActorComponent.ChildActor` (`self.RotationObject_2`))))
  (bind _asrotate_object_3 (cast `` (`ChildActorComponent.ChildActor` (`self.RotationObject_3`))))
  (bind _array (`|MakeArray` _asrotate_object _asrotate_object_2 _asrotate_object_3))
  (bind _returnvalue (`KismetArrayLibrary.Array_Length` _array))
  (set `self.number_of_rotation_objects_` (`KismetMathLibrary.Clamp` (`self.number_of_rotation_objects_`) 0 _returnvalue))
  (for _index (range _returnvalue)
    (`KismetArrayLibrary.Array_Add` (`self.rotation_objects_`) (`|GetArrayItem` _array _index)))
  (`self.SetInitialRotations`)
  (`self.SetRotationPerInteraction`))