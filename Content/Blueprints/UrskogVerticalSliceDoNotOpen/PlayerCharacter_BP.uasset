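; Player character Blueprint that manages the player's UI, camera feedback and meditation presentation.
; Gameplay, meditation and camera-fade widgets are lazily created and cached, with meditation adding breathing audio and a toggleable post-process blur, and the pause input swapping in the pause menu.
; It also plays speed-scaled head-bob camera shakes, traces the ground surface type, flags gamepad input and shares one controls pop-up with all pop-up triggers.
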(event `self.ToggleMeditationUI`
  ;[1 1 1] Toggle Meditation UI
  (`WidgetLayoutLibrary.RemoveAllWidgets`)
  (if (`self.b_meditating_`)
    (`/Game/HUD/MeditationUI_BP.ResetMeditation` (`self.meditation_widget`))
    (`self.Add Gameplay Widget`)
    (else
      (`self.Add Meditation Widget`)
      (bind _returnvalue (`self.GetSoundManager`))
      (`self.PlayBreathing` _returnvalue))))

(event `self.ToggleMeditationBlur`
  (bind _meditationblur (`self.MeditationBlur`))
  ;[1 1 1] Toggle Meditation Blur
  (if (`PostProcessComponent.bEnabled` _meditationblur)
    (set `PostProcessComponent.bEnabled` false _meditationblur)
    (else
      (set `PostProcessComponent.bEnabled` true _meditationblur))))

(event `self.ReceiveBeginPlay`
  (bind _returnvalue (`GameplayStatics.GetActorOfClass` "/Game/Blueprints/UrskogVerticalSliceDoNotOpen/PersistentVariablesCollection_BP.PersistentVariablesCollection_BP_C"))
  (set `self.mouse_sensitivity_` (`/Game/Blueprints/UrskogVerticalSliceDoNotOpen/PersistentVariablesCollection_BP.LookSensitivity` _returnvalue)))

(event `InputAction|PauseMenu` :paused true
  (params (Key :type "Key Structure"))
  (bind _returnvalue (`GameplayStatics.GetPlayerController` 0))
  (bind _pausemenu (`self.PauseMenu`))
  (:`Pressed`
    (if (`GameplayStatics.IsGamePaused`) :!label _label
      (`/Game/HUD/PauseMenu_BP.ResumeGame` _pausemenu)
      (else
        (`GameplayStatics.SetGamePaused` true)
        (`WidgetLayoutLibrary.RemoveAllWidgets`)
        (`/Engine/EditorBlueprintResources/StandardMacros.IsValid` _pausemenu
          (:`Is Valid`
            _)
          (:`Is Not Valid`
            (bind _returnvalue_2 (`|CreateWidget` "/Game/HUD/PauseMenu_BP.PauseMenu_BP_C" (`GameplayStatics.GetPlayerController` 0)))
            (set `self.PauseMenu` _returnvalue_2)))
        (`UserWidget.AddToViewport` (`self.PauseMenu`) 0)
        (`WidgetBlueprintLibrary.SetInputMode_GameAndUIEx` _returnvalue (`/Game/HUD/PauseMenu_BP.ResumeButton` (`self.PauseMenu`)))
        (set `PlayerController.bShowMouseCursor` true _returnvalue)))))

(event `InputAction|PauseMenuAlwaysEscape` :paused true
  (params (Key :type "Key Structure"))
  (:`Pressed`
    (goto _label)))

(event `self.ApplyHeadBobbing`
  (params (scale :type "Float (single-precision)"))
  (bind _returnvalue (`KismetMathLibrary.Abs` scale))
  (bind _playercameramanager (`PlayerController.PlayerCameraManager` (`GameplayStatics.GetPlayerController` 0)))
  ;[1 1 1] Head Bobbing
  (bind _returnvalue_2 (`self.GetSpeedMultiplier`))
  (bind _returnvalue_3 (`self.GetWalkSpeed`))
  (if (`self.CanJump`)
    (if (> (`CharacterMovementComponent.MaxWalkSpeed` (`self.CharacterMovement`)) (* _returnvalue_2 _returnvalue_3))
      (`PlayerCameraManager.PlayCameraShake` :`self` _playercameramanager :`ShakeClass` "/Game/Blueprints/UrskogVerticalSliceDoNotOpen/HeadBobbing_BP.HeadBobbing_BP_C" :`Scale` (* _returnvalue 2.0))
      (else
        (`PlayerCameraManager.PlayCameraShake` :`self` _playercameramanager :`ShakeClass` "/Game/Blueprints/UrskogVerticalSliceDoNotOpen/HeadBobbing_BP.HeadBobbing_BP_C" :`Scale` _returnvalue)))))

(event `self.AddPostProcessing`
  (bind _returnvalue (`AddComponent|NODE_AddPostProcessComponent-2`))
  (bind _output_get (set `self.MeditationBlur` _returnvalue))
  (set `PostProcessComponent.bEnabled` false _output_get))

(event `Key|AnyKey`
  (params (Key :type "Key Structure"))
  (:`Pressed`
    (set `self.PressedGamepadKey` (`KismetInputLibrary.Key_IsGamepadKey` Key))))

(event `self.ToggleMeditationInstructions`
  (params (is_active :type Boolean))
  (`/Engine/EditorBlueprintResources/StandardMacros.IsValid` (`self.gameplay_widget`)
    (:`Is Valid`
      (`/Game/HUD/Gameplay_BP.ToggleMeditationInstruction` (`self.gameplay_widget`) is_active))))

(event `self.InitInstructionsPopUps`
  (bind _returnvalue (`|CreateWidget` "/Game/HUD/ControlsPopUp_BP.ControlsPopUp_BP_C"))
  (`/Game/HUD/ControlsPopUp_BP.Init` _returnvalue "/Game/HUD/Controller_Instructions/PC/PC_Walk_LookAround.PC_Walk_LookAround" "/Game/HUD/Controller_Instructions/PC/Xbox_Walk_LookAround.Xbox_Walk_LookAround" "-1" "None" "None")
  (`UserWidget.AddToViewport` _returnvalue 0)
  (bind _outactors (`GameplayStatics.GetAllActorsOfClass` "/Game/Blueprints/UrskogVerticalSliceDoNotOpen/ControlsPopUpTrigger_BP.ControlsPopUpTrigger_BP_C"))
  (for _array_element _outactors
    (set `/Game/Blueprints/UrskogVerticalSliceDoNotOpen/ControlsPopUpTrigger_BP.controls_popup_` _returnvalue _array_element)))

(fn `Add Gameplay Widget`
  (bind _gameplay_widget (`self.gameplay_widget`))
  (`/Engine/EditorBlueprintResources/StandardMacros.IsValid` _gameplay_widget
    (:`Is Valid`
      (if (not (`Widget.IsInViewport` _gameplay_widget))
        (`UserWidget.AddToViewport` (`self.gameplay_widget`) 0 :!label _label)))
    (:`Is Not Valid`
      (bind _returnvalue (`|CreateWidget` "/Game/HUD/Gameplay_BP.Gameplay_BP_C"))
      (set `self.gameplay_widget` _returnvalue)
      (goto _label))))

(fn `Add Meditation Widget`
  (bind _meditation_widget (`self.meditation_widget`))
  (`/Engine/EditorBlueprintResources/StandardMacros.IsValid` _meditation_widget
    (:`Is Valid`
      (if (not (`Widget.IsInViewport` _meditation_widget))
        (`UserWidget.AddToViewport` (`self.meditation_widget`) 0 :!label _label)))
    (:`Is Not Valid`
      (bind _returnvalue (`|CreateWidget` "/Game/HUD/MeditationUI_BP.MeditationUI_BP_C"))
      (bind _output_get (set `self.meditation_widget` _returnvalue))
      (bind _returnvalue_2 (`self.GetSoundManager`))
      (set `/Game/HUD/MeditationUI_BP.sound_manager_` _returnvalue_2 _output_get)
      (`/Game/HUD/MeditationUI_BP.ResetMeditation` _output_get)
      (goto _label))))

(fn `AddCinematicWidget`
  (returns (CinematicWidget :type "/Game/HUD/CameraFade_BP Object Reference"))
  (bind _cinematicwidget (`self.CinematicWidget`))
  (bind _cinematicwidget_2 (`self.CinematicWidget`))
  (`/Engine/EditorBlueprintResources/StandardMacros.IsValid` _cinematicwidget_2
    (:`Is Valid`
      (if (`Widget.IsInViewport` _cinematicwidget_2)
        (return (`self.CinematicWidget`))
        (else
          _)))
    (:`Is Not Valid`
      (bind _returnvalue (`|CreateWidget` "/Game/HUD/CameraFade_BP.CameraFade_BP_C"))
      (set `self.CinematicWidget` _returnvalue)))
  (`UserWidget.AddToViewport` _cinematicwidget 0)
  (return _cinematicwidget))

(fn `GetPauseMenu`
  (returns (PauseMenu :type "/Game/HUD/PauseMenu_BP Object Reference"))
  (return (`self.PauseMenu`)))

(fn `RaycastToGround`
  (returns (ReturnValue :type "EPhysicalSurface Enum"))
  (bind _returnvalue (`self.K2_GetActorLocation`))
  (bind (_outhit _returnvalue_2) (`KismetSystemLibrary.LineTraceSingle` (- _returnvalue (0.0 0.0 90.0)) (- _returnvalue (0.0 0.0 150.0)) "TraceTypeQuery1"))
  (if _returnvalue_2
    (bind _output_get (set `self.ground_surface_type_` (`GameplayStatics.GetSurfaceType` _outhit)))
    (return _output_get)))

(fn `StartCinematic`
  (params (End_Cinematic :type Boolean) (`Fade time` :type "Float (double-precision)"))
  (`/Game/HUD/CameraFade_BP.Init` (`self.CinematicWidget`) End_Cinematic null `Fade time`))

(fn `UserConstructionScript`)