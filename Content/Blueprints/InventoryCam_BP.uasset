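; InventoryCam_BP is an actor that stages an object for a spinning display, apparently as an inventory preview.
; SetTargetObject stores the object and moves it to the Scene component's world location.
; While a target is held, Tick applies a slow local rotation on all three axes, scaled by delta time.
; PlaceTarget moves the object to a supplied transform and clears the target, stopping the spin.
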(event `self.ReceiveTick`
  (params (DeltaSeconds :type "Float (single-precision)"))
  (`self.RotateTarget` DeltaSeconds))

(fn `PlaceTarget`
  (params (NewTransform :type "Transform Structure"))
  (`self.K2_SetActorTransform` (`self.Target`) NewTransform false false)
  (set `self.Target` null)
  (set `self.HasTarget` false))

(fn `RotateTarget`
  (params (tick :type "Float (double-precision)"))
  (if (`self.HasTarget`)
    (`self.K2_AddActorLocalRotation` (`self.Target`) (`KismetMathLibrary.MakeRotator` (* tick 2.5) (* tick 5.0) (* tick 7.5)) false false)))

(fn `SetTargetObject`
  (params (Object :type "Actor Object Reference"))
  (bind _output_get (set `self.Target` Object))
  (`self.K2_SetActorLocation` _output_get (`SceneComponent.K2_GetComponentLocation` (`self.Scene`)) false false)
  (set `self.HasTarget` true))

(fn `UserConstructionScript`)