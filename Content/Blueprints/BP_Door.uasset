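; BP_Door is a level exit door that completes the room when a player with enough key parts reaches it.
; On overlap with its collision, it compares the PlayerCharacter_BP's key part total against the door's required amount.
; On success it plays a note sound, calls a view-target blend with no target specified, shows the WBP_CompletedRoom widget, and switches to UI-only input with a visible cursor.
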(event `self.DoorCollision.OnComponentBeginOverlap`
  (params (OverlappedComponent :type "PrimitiveComponent Object Reference") (OtherActor :type "Actor Object Reference") (OtherComp :type "PrimitiveComponent Object Reference") (OtherBodyIndex :type Integer) (bFromSweep :type Boolean) (SweepResult :type "HitResult Structure (by ref)"))
  (bind _returnvalue (`GameplayStatics.GetPlayerController` 0))
  (bind _asplayer_character_bp (cast `/Game/Blueprints/PlayerCharacter_BP` OtherActor))
  (if (>= (`/Game/Blueprints/PlayerCharacter_BP.KeyPart_TotalAmount` _asplayer_character_bp) (`self.KeyParts_RequiredAmount`))
    (`GameplayStatics.PlaySound2D` "/Game/Audio/Sound_Cues/SC_Note_5.SC_Note_5" 1.0 1.0 0.0 null null)
    (`PlayerController.SetViewTargetWithBlend` (`GameplayStatics.GetPlayerController` 0) null 0.0 "VTBlend_Linear" 0.0 false)
    (bind _returnvalue_2 (`|CreateWidget` "/Game/UI/WBP_CompletedRoom.WBP_CompletedRoom_C"))
    (`UserWidget.AddToViewport` _returnvalue_2 0)
    (`WidgetBlueprintLibrary.SetInputMode_UIOnlyEx` _returnvalue _returnvalue_2 "LockAlways")
    (set `PlayerController.bShowMouseCursor` true _returnvalue)))

(fn `UserConstructionScript`)